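; Playable spearman character Blueprint with a click-to-attack action and a zoomable camera.
; Left click, gated by IsAttacking, starts the same attack montage on the Mesh, Head, Arms, Legs and Shoulderpads components together, keeping the modular body in step.
; The OnAnimEnd_Attack event clears the gate, and the ZoomInOut axis adjusts the camera arm length within clamped limits.
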(event Custom|OnAnimEnd_Attack
  (Variables|Default|SetIsAttacking false))

(event Input|ActionEvents|InputActionMouseLeft
  (params (Key :type Key%20Structure :default "None"))
  (:Pressed
    (if (not (Variables|Default|GetIsAttacking))
      (Variables|Default|SetIsAttacking true)
      (Animation|Montage|PlayMontage (Variables|Character|GetMesh) "/Game/Toon_RTS_Units_Barbarians/Animations/Spearman/Anim_spearman_07_attack_Montage.Anim_spearman_07_attack_Montage"
        (:then
          (Animation|Montage|PlayMontage (Variables|Default|GetHead) "/Game/Toon_RTS_Units_Barbarians/Animations/Spearman/Anim_spearman_07_attack_Montage.Anim_spearman_07_attack_Montage"
            (:then
              (Animation|Montage|PlayMontage (Variables|Default|GetArms) "/Game/Toon_RTS_Units_Barbarians/Animations/Spearman/Anim_spearman_07_attack_Montage.Anim_spearman_07_attack_Montage"
                (:then
                  (Animation|Montage|PlayMontage (Variables|Default|GetLegs) "/Game/Toon_RTS_Units_Barbarians/Animations/Spearman/Anim_spearman_07_attack_Montage.Anim_spearman_07_attack_Montage"
                    (:then
                      (Animation|Montage|PlayMontage (Variables|Default|GetShoulderpads) "/Game/Toon_RTS_Units_Barbarians/Animations/Spearman/Anim_spearman_07_attack_Montage.Anim_spearman_07_attack_Montage"))))))))))))

(event Input|AxisEvents|InputAxisZoomInOut
  (params (AxisValue :type Float%20%28single-precision%29))
  (bind _cameraarm (Variables|Default|GetCameraArm))
  ;[1 1 1] Camera
  (Variables|/Script/Engine.SpringArmComponent|SetTargetArmLength _cameraarm (Math|Float|Clamp(Float) (+ (* AxisValue 3e+01) (Variables|/Script/Engine.SpringArmComponent|GetTargetArmLength _cameraarm)) 2e+02 1e+03)))

(fn ConstructionScript)