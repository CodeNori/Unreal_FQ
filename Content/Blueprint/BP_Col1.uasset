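; BP_Col1 is a collision test actor that lights up on overlap and forms a detection line with other instances of itself.
; Begin overlap prints both actor names and shows the PointLight, and end overlap hides it.
; Each tick, a debug-drawn Pawn object trace runs between the first two BP_Col1 instances found at BeginPlay.
; A hit Character's BodyColor material parameter turns red; with no hit, the player's is set to OrgBodyColor.
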(event EventBeginPlay
  (bind _outactors (Actor|GetAllActorsOfClass "BP_Col1_C"))
  (Variables|Default|SetLines _outactors))

(event Collision|EventActorBeginOverlap
  (params (OtherActor :type Actor%20Object%20Reference))
  (Development|PrintString (Utilities|String|Append (Utilities|GetDisplayName self) "== " (Utilities|GetDisplayName OtherActor)))
  (Rendering|SetVisibility (Variables|Default|GetPointLight) true false))

(event EventTick
  (params (DeltaSeconds :type Float%20%28single-precision%29))
  (bind _lines (Variables|Default|GetLines))
  (bind (_outhit _returnvalue) (Collision|LineTraceForObjects (Transformation|GetActorLocation (Utilities|Array|Get(acopy) _lines)) (Transformation|GetActorLocation (Utilities|Array|Get(acopy) _lines 1)) (Utilities|Array|MakeArray "ObjectTypeQuery3") false (Variables|Default|GetLines) "ForOneFrame" true "(R=0.000000,G=1.000000,B=0.000000,A=1.000000)" "(R=1.000000,G=0.000000,B=0.000000,A=1.000000)" 0.0))
  (if _returnvalue
    (bind _ascharacter (Utilities|Casting|CastToCharacter (.HitActor (Collision|BreakHitResult _outhit))))
    (Rendering|Material|SetVectorParameterValueonMaterials (Variables|/Script/Engine.Character|GetMesh _ascharacter) "BodyColor" "1.000000, 0, 0")
    (else
      (bind _ascharacter_2 (Utilities|Casting|CastToCharacter (Game|GetPlayerCharacter 0)))
      (Rendering|Material|SetVectorParameterValueonMaterials (Variables|/Script/Engine.Character|GetMesh _ascharacter_2) "BodyColor" (Math|Conversions|ToVector(LinearColor) (Variables|Default|GetOrgBodyColor))))))

(event Collision|EventActorEndOverlap
  (params (OtherActor :type Actor%20Object%20Reference))
  (Rendering|SetVisibility (Variables|Default|GetPointLight) false false))

(fn ConstructionScript)